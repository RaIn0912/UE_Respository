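; WallLight_BP is an interactable wall light that works as one piece of a puzzle to open a mechanism door.
; Box overlap by ThirdPersonCharacter toggles input and a gate, showing a text prompt while the light is unlit.
; Pressing E turns on the spotlight and marks it open, then checks every WallLight_BP in the level.
; When all are lit, a "ce" console command fires the door-opening event (开启机关门), avoiding a direct reference.
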(event OnComponentBeginOverlap(Box)
  (params (OverlappedComponent :type Primitive%20Component%20Object%20Reference) (OtherActor :type Actor%20Object%20Reference) (OtherComp :type Primitive%20Component%20Object%20Reference) (OtherBodyIndex :type Integer) (bFromSweep :type Boolean) (SweepResult :type Hit%20Result%20Structure%20%28by%20ref%29))
  (Utilities|Casting|CastToThirdPersonCharacter OtherActor)
  (if (not (Variables|Default|GetisOpen))
    (Input|EnableInput (Game|GetPlayerController 0))
    (Rendering|SetVisibility (Variables|Default|GetTextRender) true false)
    (Utilities|FlowControl|Gate true) ; enters at Open
  ))

(event OnComponentEndOverlap(Box)
  (params (OverlappedComponent :type Primitive%20Component%20Object%20Reference) (OtherActor :type Actor%20Object%20Reference) (OtherComp :type Primitive%20Component%20Object%20Reference) (OtherBodyIndex :type Integer))
  (Utilities|Casting|CastToThirdPersonCharacter OtherActor)
  (Input|DisableInput (Game|GetPlayerController 0))
  (Rendering|SetVisibility (Variables|Default|GetTextRender) false false)
  (Utilities|FlowControl|Gate true) ; enters at Close
)

(event Input|KeyboardEvents|E
  (params (Key :type Key%20Structure :default "None"))
  (:Pressed
    (Utilities|FlowControl|Gate true
      (:Exit
        (Rendering|SetVisibility (Variables|Default|GetSpotLight) true false)
        (Rendering|SetVisibility (Variables|Default|GetTextRender) false false)
        (Variables|Default|SetisOpen true)
        (bind _outactors (Actor|GetAllActorsOfClass "WallLight_BP_C"))
        (bind _array_element (Utilities|Array|ForEachLoopwithBreak _outactors :!label _label)
          (:LoopBody
            (if (Variables|WallLight_BP_C|GetisOpen _array_element)
              (Variables|Default|SetisAllOpen true)
              (else
                (Variables|Default|SetisAllOpen false)
                (goto _label Break))))
          (:Completed
            (if (Variables|Default|GetisAllOpen)
              (Development|ExecuteConsoleCommand "ce 开启机关门" 0))))))))

(fn ConstructionScript)